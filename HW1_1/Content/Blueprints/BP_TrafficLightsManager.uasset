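; Traffic light manager that cycles two groups of lights through the colors in a ColorSettings map, starting at BeginPlay.
; RecolorLoop calls ChangeColor to apply each group's current color by its own index, wrapping at the end.
; Each group's output branch waits in a Delay timed by color name via GetDuration, increments that index and re-enters the shared loop.
; ChangeColorSecond is an uncalled single-group variant.
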(event Custom|Recolor
  (bind _keys (Utilities|Map|Keys (.colormap (Variables|Default|GetColorSettings))))
  (Variables|Default|SetColorNameArray _keys)
  (CallFunction|RecolorLoop))

(event Custom|RecolorLoop
  (Utilities|ChangeColor (Variables|Default|GetTrafficLightsGroupA) (Variables|Default|GetTrafficLightsGroupB)
    (:LightTrafficGroupA
      (Utilities|FlowControl|Sequence
        (:then_0
          (bind _durationvar (Utilities|GetDuration (Variables|Default|GetColorIndexGroupA))))
        (:then_1
          (Utilities|FlowControl|Delay _durationvar)
          (Math|Integer|IncrementInt (Variables|Default|GetColorIndexGroupA)
            (:%20%20
              (CallFunction|RecolorLoop))))))
    (:LightTrafficGroupB
      (Utilities|FlowControl|Sequence
        (:then_0
          (bind _durationvar_2 (Utilities|GetDuration (Variables|Default|GetColorIndexSecondGroupB))))
        (:then_1
          (Utilities|FlowControl|Delay _durationvar_2)
          (Math|Integer|IncrementInt (Variables|Default|GetColorIndexSecondGroupB)
            (:%20%20
              (CallFunction|RecolorLoop))))))))

(event EventBeginPlay
  (CallFunction|Recolor))

(fn ConstructionScript)